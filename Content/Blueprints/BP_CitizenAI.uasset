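; Citizen NPC Blueprint that wanders endlessly between random reachable navmesh points, starting on BeginPlay.
; It sets a forward walk animation once, waits a random moment, then issues AI MoveTo within a very large radius.
; The loop re-issues moves on timed delays from the immediate output, without waiting for arrival.
; IsMoving is set true only before the loop and cleared during the first cycle.
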(event Custom|NPC_Roam
  (Components|Animation|SetAnimation (Variables|Character|GetMesh) "/Game/Characters/Mannequins/Animations/Quinn/MF_Walk_Fwd.MF_Walk_Fwd")
  (Utilities|FlowControl|Delay (Math|Random|RandomFloatinRange 1.0 3.0))
  (Variables|Default|SetisMoving? true)
  (for _index (range 0 0) :!label _label
    (AI|AIMoveTo self (.RandomLocation (AI|Navigation|GetRandomReachablePointinRadius (Transformation|GetActorLocation) 1e+05 0 0)) 0 5.0 false
      (:then
        (Utilities|FlowControl|Delay (Math|Random|RandomFloatinRange 1.0 3.0))
        (Variables|Default|SetisMoving? false)
        (Utilities|FlowControl|Delay 5.0)
        (goto _label)))))

(event EventBeginPlay
  (CallFunction|NPCRoam))

(fn ConstructionScript)