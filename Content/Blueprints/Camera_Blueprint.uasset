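; Security camera that raises an alarm when it spots the player and calls in guards.
; AI Perception detects the third-person character, plays a 2D alarm, then waits one second; the follow-up visibility check is hardwired true.
; It then sends every BP_BrianGuard sharing its GroupID to investigate the player's current location, passing along its PatrolPoints.
; The PawnSensing sight event is empty, and debug draw and print nodes are disconnected.
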(event OnSeePawn(PawnSensing)
  (params (Pawn :type Pawn%20Object%20Reference)))

(event OnTargetPerceptionUpdated(AIPerception)
  (params (Actor :type Actor%20Object%20Reference) (Stimulus :type AI%20Stimulus%20Structure))
  (bind _asbp_third_person_character (Utilities|Casting|CastToBP_ThirdPersonCharacter Actor))
  (if (.bSuccessfullySensed (Utilities|Struct|BreakAIStimulus Stimulus)) ; did we start/stop seeing the plaayer
    (Audio|PlaySound2D "/Game/Sound/alarm-no3-14864.alarm-no3-14864" 1.0 1.0 0.0 0 0)
    (Utilities|FlowControl|Delay 1.0)
    (if true ; after delay, do we still see the player
      (bind _outactors (Actor|GetAllActorsOfClass "/Game/Blueprints/BP_BrianGuard.BP_BrianGuard_C"))
      (for _array_element _outactors
        (if (== (Variables|Default|GetGroupID) (Variables|/Game/Blueprints/BP_BrianGuard.BP_BrianGuard_C|GetGroupID _array_element))
          (Default|Investigate _array_element (Transformation|GetWorldLocation (Variables|/Script/Engine.Character|GetCapsuleComponent (Game|GetPlayerCharacter 0))) (Variables|Default|GetPatrolPoints)))))))

(event EventBeginPlay
  (Components|Activation|Activate (Variables|Default|GetPawnSensing) false))

(event Collision|EventActorBeginOverlap
  (params (OtherActor :type Actor%20Object%20Reference)))

(event EventTick
  (params (DeltaSeconds :type Float%20%28single-precision%29)))

(fn ConstructionScript)