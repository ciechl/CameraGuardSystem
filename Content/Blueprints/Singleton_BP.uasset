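; Game instance singleton that saves, loads and deletes per-level records of collected coins, using the level name as save slot.
; Load clears AlreadyCollectedObjects, then destroys the saved PickedUpCoins actors without copying them back into that array.
; Save overwrites the slot's Save_Objects_BP coin list with AlreadyCollectedObjects, creating the save object if needed.
; DeleteSave ignores its existence check and always attempts deletion.
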(event Custom|Load
  ;[0 0.4171 1] LoadGame
  (Utilities|FlowControl|Delay 0.2)
  (bind _returnvalue (Game|GetCurrentLevelName true))
  (Utilities|Array|Clear (Variables|Default|GetAlreadyCollectedObjects)) ; new level, clear out this playthrough's array of collected objects
  (Development|PrintString (Utilities|String|Append "Starting load in level " _returnvalue ", wish me luck!"))
  (bind _returnvalue_2 (SaveGame|DoesSaveGameExist _returnvalue))
  (if _returnvalue_2
    (bind _returnvalue_3 (SaveGame|LoadGamefromSlot _returnvalue))
    (bind _assave_objects_bp (Utilities|Casting|CastToSave_Objects_BP _returnvalue_3))
    (Variables|Default|SetAs%20Save%20Objects%20BP _assave_objects_bp) ; reference to save game object
    (for _array_element (Variables|/Game/Blueprints/Save_Objects_BP.Save_Objects_BP_C|GetPickedUpCoins _assave_objects_bp)
      (Actor|DestroyActor _array_element))))

(event Custom|DeleteSave
  (Development|PrintString "Hello")
  (bind _returnvalue (Game|GetCurrentLevelName true))
  (SaveGame|DoesSaveGameExist _returnvalue)
  (if true
    (SaveGame|DeleteGameinSlot _returnvalue)
    (Development|PrintString "Save detector")
    (else
      (Development|PrintString "No save game exists!"))))

(event Custom|Save
  (Development|PrintString "Starting save")
  (bind _returnvalue (Game|GetCurrentLevelName true))
  (bind _returnvalue_2 (SaveGame|DoesSaveGameExist _returnvalue))
  (if _returnvalue_2
    (bind _returnvalue_3 (SaveGame|LoadGamefromSlot _returnvalue))
    (Variables|Default|SetSaver%20Subclass _returnvalue_3)
    (else
      (bind _returnvalue_4 (SaveGame|CreateSaveGameObject "/Game/Blueprints/Save_Objects_BP.Save_Objects_BP_C"))
      (Variables|Default|SetSaver%20Subclass _returnvalue_4)))
  (bind _assave_objects_bp (Utilities|Casting|CastToSave_Objects_BP (Variables|Default|GetSaver%20Subclass))
    (:then
      (Variables|/Game/Blueprints/Save_Objects_BP.Save_Objects_BP_C|SetPickedUpCoins _assave_objects_bp (Variables|Default|GetAlreadyCollectedObjects)) ; save game matches what the game instance (singleton) has
      (bind _returnvalue_5 (Game|GetCurrentLevelName true))
      (SaveGame|SaveGametoSlot _assave_objects_bp _returnvalue_5)
      (Development|PrintString "save successful"))
    (:CastFailed
      (Development|PrintString "Cast failed in save game"))))