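; Enemy AI pawn (KillBoss) that patrols, investigates, chases on sight and catches the player.
; BeginPlay saves the start location, starts patrolling and loops a short-delay distance check that calls Caught on the player character when close.
; Investigate takes a destination and new patrol points, then patrols them before returning to start.
; PawnSensing triggers Chase toward the seen pawn's location, resuming patrol when the move ends; optional debug text shows the state.
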(event OnSeePawn(PawnSensing)
  (params (Pawn :type Pawn%20Object%20Reference))
  (CallFunction|Chase))

(event Custom|Investigate
  (params (Destination :type Vector) (PatrolPoints :type Array%20of%20Actor%20Object%20References))
  (if (Variables|Default|GetDebugging)
    (Rendering|Components|TextRender|SetText (Variables|Default|GetTextRender) (Utilities|Text|ToText(String) "Investigate")))
  (Variables|Default|SetPatrolPoints PatrolPoints) ; Get camera patrol points
  (Variables|Default|SetIndex 0) ; Reset patrol point index
  (AI|AIMoveTo self Destination 0 1e+02 false
    (:OnSuccess
      (Utilities|FlowControl|Delay 2.0)
      (if (not (Variables|Default|GetChasing)) ; IF not chasing player, go patrol
        (CallFunction|Patrol)))))

(event Custom|ReturnToStation
  (if (Variables|Default|GetDebugging)
    (Rendering|Components|TextRender|SetText (Variables|Default|GetTextRender) (Utilities|Text|ToText(String) "Return")))
  (AI|AIMoveTo self (Variables|Default|GetStartLocation) 0 1e+02 false))

(event Custom|Patrol
  (if (Variables|Default|GetDebugging)
    (Rendering|Components|TextRender|SetText (Variables|Default|GetTextRender) (Utilities|Text|ToText(String) "Patrol")))
  (AI|AIMoveTo self "0, 0, 0" (Utilities|Array|Get(acopy) (Variables|Default|GetPatrolPoints) (Variables|Default|GetIndex)) 1e+02 false :!label _label
    (:OnSuccess
      _)
    (:OnFail
      _))
  (Utilities|FlowControl|Delay 3.0)
  (Math|Integer|IncrementInt (Variables|Default|GetIndex)
    (:%20%20
      (if (not (Variables|Default|GetChasing)) ; If chasing player, stop patrol
        (if (>= (Variables|Default|GetIndex) (Utilities|Array|Length (Variables|Default|GetPatrolPoints)))
          (CallFunction|ReturntoStation)
          (else
            (goto _label)))))))

(event Custom|Chase
  (if (Variables|Default|GetDebugging)
    (Rendering|Components|TextRender|SetText (Variables|Default|GetTextRender) (Utilities|Text|ToText(String) "Chase")))
  (Variables|Default|SetChasing true)
  (bind _movementresult (AI|AIMoveTo self (Transformation|GetActorLocation (stale OnSeePawn(PawnSensing) Pawn)) 0 5e+01 false)
    (:OnSuccess
      _)
    (:OnFail
      _))
  (switch Utilities|FlowControl|Switch|SwitchonEPathFollowingResult _movementresult
    (:Success
      (Development|PrintString "GOT YOU"))
    (:Blocked
      _)
    (:OffPath
      _)
    (:Invalid
      _))
  (Variables|Default|SetChasing false)
  (CallFunction|Patrol))

(event EventBeginPlay
  (Variables|Default|SetStartLocation (Transformation|GetWorldLocation (Variables|Collision|GetCapsuleComponent))) ; save starting location
  (CallFunction|Patrol)
  (Utilities|FlowControl|Delay 0.2 :!label _label)
  (if (<= (Math|Vector|Distance(Vector) (Transformation|GetWorldLocation (Variables|Collision|GetCapsuleComponent)) (Transformation|GetWorldLocation (Variables|/Script/Engine.Character|GetCapsuleComponent (Game|GetPlayerCharacter 0)))) 1e+02)
    (Development|PrintString "Hello")
    (bind _asbp_third_person_character (Utilities|Casting|CastToBP_ThirdPersonCharacter (Game|GetPlayerCharacter 0)))
    (Default|Caught _asbp_third_person_character)
    (goto _label)
    (else
      (goto _label))))

(fn ConstructionScript)