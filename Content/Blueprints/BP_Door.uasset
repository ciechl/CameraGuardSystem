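; BP_Door is a door that opens by removing itself once the player has more than six kills.
; Every Tick it finds BP_ThirdPersonCharacter with GetActorOfClass and checks its Kills count, then plays a door-open sound and destroys itself.
; The Box overlap event is empty, leaving disconnected logic that would briefly show a UI_KillsRemain widget.
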(event OnComponentBeginOverlap(Box)
  (params (OverlappedComponent :type Primitive%20Component%20Object%20Reference) (OtherActor :type Actor%20Object%20Reference) (OtherComp :type Primitive%20Component%20Object%20Reference) (OtherBodyIndex :type Integer) (bFromSweep :type Boolean) (SweepResult :type Hit%20Result%20Structure%20%28by%20ref%29)))

(event EventBeginPlay)

(event Collision|EventActorBeginOverlap
  (params (OtherActor :type Actor%20Object%20Reference)))

(event EventTick
  (params (DeltaSeconds :type Float%20%28single-precision%29))
  (bind _returnvalue (Actor|GetActorOfClass "/Game/ThirdPerson/Blueprints/BP_ThirdPersonCharacter.BP_ThirdPersonCharacter_C"))
  (bind _asbp_third_person_character (Utilities|Casting|CastToBP_ThirdPersonCharacter _returnvalue))
  (if (> (Variables|/Game/ThirdPerson/Blueprints/BP_ThirdPersonCharacter.BP_ThirdPersonCharacter_C|GetKills _asbp_third_person_character) 6)
    (Audio|PlaySound2D "/Game/Sound/door-open-107728.door-open-107728" 1.0 1.0 0.0 0 0)
    (Actor|DestroyActor self)))

(fn ConstructionScript)