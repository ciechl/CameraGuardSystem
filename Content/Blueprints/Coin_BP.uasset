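; Coin_BP is a collectible coin pickup that spins in the level and adds to the player's score when touched.
; Tick rotates the root component in yaw at RotateSpeed, scaled by delta time.
; Any overlap with its Sphere increments Score on the Singleton_BP game instance, records the coin in AlreadyCollectedObjects, then destroys the actor.
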(event OnComponentBeginOverlap(Sphere)
  (params (OverlappedComponent :type Primitive%20Component%20Object%20Reference) (OtherActor :type Actor%20Object%20Reference) (OtherComp :type Primitive%20Component%20Object%20Reference) (OtherBodyIndex :type Integer) (bFromSweep :type Boolean) (SweepResult :type Hit%20Result%20Structure%20%28by%20ref%29))
  (bind _assingleton_bp (Utilities|Casting|CastToSingleton_BP (Game|GetGameInstance)))
  (Math|Integer|IncrementInt (Variables|/Game/Blueprints/Singleton_BP.Singleton_BP_C|GetScore _assingleton_bp)
    (:%20%20
      (Utilities|Array|Add (Variables|/Game/Blueprints/Singleton_BP.Singleton_BP_C|GetAlreadyCollectedObjects _assingleton_bp) self)
      (Actor|DestroyActor))))

(event EventTick
  (params (DeltaSeconds :type Float%20%28single-precision%29))
  (Transformation|AddLocalRotation (Variables|Default|GetDefaultSceneRoot) (Math|Rotator|MakeRotator 0.0 0.0 (* DeltaSeconds (Variables|Default|GetRotateSpeed))) false false))

(fn ConstructionScript)